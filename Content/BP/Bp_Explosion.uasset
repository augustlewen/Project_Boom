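; One-shot explosion actor that blasts nearby objects as soon as it spawns, then destroys itself after a short delay.
; On BeginPlay, a sphere overlap matching the RadialForce radius sends BlastMessage to static and dynamic world actors it finds.
; If the player character is among them and jumping, its velocity is zeroed before the radial impulse fires alongside the explosion sound.
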(event EventBeginPlay
  (bind _returnvalue (Game|GetPlayerCharacter 0))
  (bind _radialforce (Variables|Default|GetRadialForce))
  (bind _returnvalue_2 (Transformation|GetWorldLocation _radialforce))
  (Utilities|FlowControl|Sequence
    (:then_0
      ;[0.6829 0.6305 1] Blast Event is called for any blastable actors within the explosion range
      (bind _outactors (Collision|SphereOverlapActors _returnvalue_2 (Variables|/Script/Engine.RadialForceComponent|GetRadius _radialforce) (Utilities|Array|MakeArray "ObjectTypeQuery1" "ObjectTypeQuery2") 0))
      (for _array_element _outactors
        (Class|BpInterface|Blast(Message) _array_element)
        (if (== _array_element _returnvalue)
          (bind _asbp_player (Utilities|Casting|CastToBP_Player _returnvalue))
          (if (Variables|/Game/BP/BP_Player.BP_Player_C|GetisJumping _asbp_player)
            (Variables|/Script/Engine.MovementComponent|SetVelocity (Variables|/Script/Engine.Character|GetCharacterMovement _asbp_player) "0, 0, 0")))))
    (:then_1
      ;[1 0.2471 0] Emit a radial force to nearby objects
      (Class|RadialForceComponent|FireImpulse (Variables|Default|GetRadialForce))
      (Audio|PlaySoundatLocation "/Game/Assets/Sounds/Explosion_Cue.Explosion_Cue" _returnvalue_2 "0, 0, 0" 1.0 1.0 0.0 0 0 0))
    (:then_2
      ;[1 0 0.04149] Destroy Self After short delay
      (Utilities|FlowControl|Delay 0.25)
      (Actor|DestroyActor))))

(fn ConstructionScript)