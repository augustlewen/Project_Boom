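; BP_Bomb is a throwable C4 charge that sticks to whatever it hits and can be detonated.
; On BeginPlay it launches the physics-driven C4 component forward with an impulse and adds the player to an ignore list.
; On hit it disables physics and collision, aligns to the surface using a mirrored-vector look-at, and attaches to the hit component.
; The Explode event spawns BP_Explosion at the C4's transform and destroys the bomb.
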(event OnComponentHit(C4)
  (params (HitComponent :type Primitive%20Component%20Object%20Reference) (OtherActor :type Actor%20Object%20Reference) (OtherComp :type Primitive%20Component%20Object%20Reference) (NormalImpulse :type Vector :default "0, 0, 0") (Hit :type Hit%20Result%20Structure%20%28by%20ref%29))
  (bind (_bblockinghit _binitialoverlap _time _distance _location _impactpoint _normal) (Collision|BreakHitResult Hit))
  (bind _c4 (Variables|Default|GetC4))
  ;[0.08091 1 0.4591] Hit Component: Stick to surface and change rotation to allign the surface
  (Physics|SetSimulatePhysics _c4 false)
  (Collision|SetCollisionEnabled (Variables|Default|GetC4) "NoCollision")
  (Transformation|SetWorldRotation (Variables|Default|GetC4) (Math|Rotator|FindLookatRotation (Transformation|GetWorldLocation _c4) (Math|Vector|MirrorVectorbyNormal _location _normal)) false false)
  (Transformation|AddLocalRotation (Variables|Default|GetC4) (Math|Rotator|MakeRotator 0.0 9e+01 0.0) false false)
  (Transformation|AttachComponentToComponent (Variables|Default|GetC4) OtherComp "None" "KeepWorld" "KeepRelative" "KeepWorld" true))

(event Custom|Explode
  ;[1 0.1112 0] Explode Event: Spawn Explosion
  (Game|SpawnActorfromClass "/Game/BP/Bp_Explosion.BP_Explosion_C" (Transformation|GetWorldTransform (Variables|Default|GetC4)) "Undefined" 0 0)
  (Actor|DestroyActor))

(event EventBeginPlay
  ;[0.3524 0.8799 1] Throw C4 in the Forward direction
  (Physics|AddImpulse (Variables|Default|GetC4) (* (Math|Vector|GetForwardVector (Variables|Default|GetDefaultSceneRoot)) 2e+04) "None" false)
  ;[0.8274 0.333 1] Add player to actors to ignore array
  (Utilities|Array|Add (Variables|Default|GetActorsToIgnore) (Game|GetPlayerCharacter 0)))

(fn ConstructionScript)