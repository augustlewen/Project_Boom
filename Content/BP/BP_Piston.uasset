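; Piston Blueprint whose pillar extends or retracts along its local Z axis when switched on or off.
; On and Off set the target length and swap a pillar material; On also plays a sound at the recorded start position.
; Both restart a timeline that eases the pillar toward the target with FInterpTo, using a fixed delta time, so motion depends on update rate.
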(event Custom|Ascend/Descend
  ;[1 0.6429 0] Ascend / Descend Event
  (Timeline|Timeline PlayFromStart
    (:Update
      (Transformation|SetRelativeLocation (Variables|Default|GetPillar) (Math|Vector|MakeVector 0.0 0.0 (Math|Interpolation|FInterpTo (.z (Variables|/Script/Engine.SceneComponent|GetRelativeLocation (Variables|Default|GetPillar))) (Variables|Default|GetTarget%20Length) 0.5 0.05)) false false))))

(event EventOn
  ;[1 0.08657 0] Pillar On / Off Event -> Set Target Height & Material
  (Variables|Default|SetTarget%20Length (Variables|Default|GetExtend%20Length))
  (Rendering|Material|SetMaterial (Variables|Default|GetPillar) 2 (Variables|Default|GetMaterialOn))
  (Audio|PlaySoundatLocation "/Game/Assets/Sounds/Cue_Piston.Cue_Piston" (Variables|Default|GetStartPosition) "0, 0, 0" 1.0 1.0 0.0 0 0 0 0)
  (CallFunction|Ascend/Descend))

(event EventOff
  ;[1 0.08657 0] Pillar On / Off Event -> Set Target Height & Material
  (Variables|Default|SetTarget%20Length 0.0)
  (Rendering|Material|SetMaterial (Variables|Default|GetPillar) 2 (Variables|Default|GetMaterialOff))
  (CallFunction|Ascend/Descend))

(event EventBeginPlay
  ;[0.4809 1 0.1012] Set Start Height Variable
  (Variables|Default|SetStartPosition (Transformation|GetWorldLocation (Variables|Default|GetPillar))))

(fn ConstructionScript)