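; Blast module actor that, when triggered, temporarily activates a set of connected actors.
; The Blast event ignores retriggers while active, sends OnMessage to each connected actor and swaps the module mesh to its lit material.
; After the ActiveTime delay it sends OffMessage to the same actors, clears the active flag and restores the off material.
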(event EventBlast
  ;[1 0.5777 0] Activate all connected actors
  (if (not (Variables|Default|GetisActivated))
    (Variables|Default|SetisActivated true)
    (for _array_element (Variables|Default|GetConnectedActors)
      (Class|BpInterface|On(Message) _array_element))
    (Utilities|FlowControl|Sequence
      (:then_0
        (Rendering|Material|SetMaterial (Variables|Default|GetModule) 1 (Variables|Default|GetM_On)))
      (:then_1
        ;[1 0.1388 0] Deactivate all connected actors
        (Utilities|FlowControl|Delay (Variables|Default|GetActiveTime))
        (for _array_element_2 (Variables|Default|GetConnectedActors)
          (Class|BpInterface|Off(Message) _array_element_2))
        (Variables|Default|SetisActivated false)
        (Rendering|Material|SetMaterial (Variables|Default|GetModule) 1 (Variables|Default|GetM_Off))))))

(fn ConstructionScript)